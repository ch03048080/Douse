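; BP_EnemySpawn is an enemy spawner that places BPMaster_Enemies actors along the edges of a square area centered on the world origin.
; BeginPlay starts a looping one-second timer, presumably bound to SpawnEnemies.
; SpawnEnemies randomly picks one of four edges and a random point along it at a fixed height, then spawns an enemy there.
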(event Custom|SpawnEnemies
  (switch int (Math|Random|RandomIntegerinRange 1 4)
    (:1
      (Variables|Default|SetLocation (Math|Vector|MakeVector (Math|Random|RandomFloatinRange -1.95e+03 1.95e+03) 1.95e+03 88.0)))
    (:2
      (Variables|Default|SetLocation (Math|Vector|MakeVector (Math|Random|RandomFloatinRange -1.95e+03 1.95e+03) -1.95e+03 88.0)))
    (:3
      (Variables|Default|SetLocation (Math|Vector|MakeVector 1.95e+03 (Math|Random|RandomFloatinRange -1.95e+03 1.95e+03) 88.0)))
    (:4
      (Variables|Default|SetLocation (Math|Vector|MakeVector -1.95e+03 (Math|Random|RandomFloatinRange -1.95e+03 1.95e+03) 88.0))))
  (Game|SpawnActorfromClass "/Game/Blueprints/Enemies/BPMaster_Enemies.BPMaster_Enemies_C" (Math|Transform|MakeTransform (Variables|Default|GetLocation) "0, 0, 0" "1.000000,1.000000,1.000000") "Undefined" 0 0))

(event EventBeginPlay
  (Utilities|Time|SetTimerbyEvent (EventDispatchers|CreateEvent :!event Custom|SpawnEnemies) 1.0 true))

(event Collision|EventActorBeginOverlap
  (params (OtherActor :type Actor%20Object%20Reference)))

(event EventTick
  (params (DeltaSeconds :type Float%20%28single-precision%29)))

(fn ConstructionScript)