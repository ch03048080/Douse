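; BP_Pickup is a coin pickup that spins continuously and grants coin experience when a PlayerCharacter overlaps its collision sphere.
; A looping timeline drives the yaw spin, while a once-only overlap timeline shrinks the coin and lerps it from its spawn point to its own current location.
; When that finishes, it awards BaseValue, plays a sound and destroys itself.
; An unconnected BP_Player variant instead moves the coin toward the player.
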(event OnComponentBeginOverlap(CollisionSphere)
  (params (OverlappedComponent :type Primitive%20Component%20Object%20Reference) (OtherActor :type Actor%20Object%20Reference) (OtherComp :type Primitive%20Component%20Object%20Reference) (OtherBodyIndex :type Integer) (bFromSweep :type Boolean) (SweepResult :type Hit%20Result%20Structure%20%28by%20ref%29))
  ;[1 1 1] 코멘트
  (bind _asplayer_character (Utilities|Casting|CastToPlayerCharacter OtherActor))
  (Variables|Default|SetAs%20Player%20Character _asplayer_character)
  (Utilities|FlowControl|DoOnce false
    (:Completed
      (bind _alpha (Timeline|타임라인 PlayFromStart) ; ?
        (:Update
          (Transformation|SetActorLocation (Math|Vector|Lerp(Vector) (Variables|Default|GetStartlingPickupLocation) (Transformation|GetActorLocation) _alpha) false false)
          (Transformation|SetActorScale3D (Math|Vector|Lerp(Vector) "1.000000,1.000000,1.000000" "0, 0, 0" _alpha)))
        (:Finished
          (Class|PlayerCharacter|AddCoinExpericence (Variables|Default|GetAs%20Player%20Character) (Variables|Default|GetBaseValue))
          (Audio|PlaySoundatLocation "/Engine/VREditor/Sounds/VR_open.VR_open" (Transformation|GetActorLocation) "0, 0, 0" 1.0 1.0 0.0 0 0 0 0)
          (Actor|DestroyActor))))))

(event EventBeginPlay
  ;[0.3021 0.3021 0.3021] Start spin the coin when it is spawned
  (Variables|Default|SetStartlingPickupLocation (Transformation|GetActorLocation))
  (bind _timer (Timeline|Timeline PlayFromStart)
    (:Update
      (Transformation|SetActorRotation (Math|Rotator|MakeRotator 0.0 0.0 (Math|Float|Lerp 0.0 3.6e+02 _timer))))
    (:Finished
      (Timeline|Timeline PlayFromStart))))

(fn ConstructionScript)