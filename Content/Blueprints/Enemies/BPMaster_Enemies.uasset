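; Master enemy Blueprint for dragon-type monsters that chase the player and deal contact damage on a short cooldown.
; BeginPlay loops AIMoveTo toward the player and caches the health widget.
; Spell hits apply randomized damage, update the health bar, show damage numbers and flash emissive through a timeline-driven dynamic material.
; Death disables movement and collision, drops a pickup by enemy type, plays a montage, then destroys the actor and increments the player's kill count.
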(event OnComponentBeginOverlap(DragonCollision)
  (params (OverlappedComponent :type Primitive%20Component%20Object%20Reference) (OtherActor :type Actor%20Object%20Reference) (OtherComp :type Primitive%20Component%20Object%20Reference) (OtherBodyIndex :type Integer) (bFromSweep :type Boolean) (SweepResult :type Hit%20Result%20Structure%20%28by%20ref%29))
  ;[1 1 1] C++ 변환 완료
  (bind _asbp_player_character (Utilities|Casting|CastToBP_PlayerCharacter OtherActor))
  (Utilities|FlowControl|DoOnce false :!label _label
    (:Completed
      (Class|PlayerCharacter|GetHurtandUpdateHealth _asbp_player_character (Variables|Default|GetEnemy%20Damage))
      (Utilities|FlowControl|Delay 0.8)
      (goto _label Reset))))

(event Custom|EnemyFlashingEffect
  (bind _flashalpha (Timeline|FlashingTimer PlayFromStart)
    (:Update
      (Rendering|Material|SetScalarParameterValue (Variables|Default|GetRef_Material) "Emissive" _flashalpha :!class /Script/Engine.MaterialInstanceDynamic))))

(event EventBeginPlay
  (bind _aswbp_enemy_health (Utilities|Casting|CastToWBP_EnemyHealth (UserInterface|GetWidget (Variables|Default|GetWidget))))
  (Variables|Default|SetAs%20WBP%20Enemy%20Health _aswbp_enemy_health)
  (AI|AIMoveTo self "0, 0, 0" (Game|GetPlayerCharacter 0) 5e+01 false :!label _label
    (:OnSuccess
      (Utilities|FlowControl|Delay 1.0)
      (goto _label))))

(event Collision|EventActorBeginOverlap
  (params (OtherActor :type Actor%20Object%20Reference)))

(event EventTick
  (params (DeltaSeconds :type Float%20%28single-precision%29)))

(event EventSpellCollisionEvent
  (params (SpellDamageInput :type Float%20%28double-precision%29))
  (bind _returnvalue (Math|Random|RandomFloatinRange -5.0 5.0))
  (bind _returnvalue_2 (Transformation|GetActorTransform))
  (bind _returnvalue_3 (+ SpellDamageInput _returnvalue))
  (bind _output_get (Variables|Default|SetEnemyCurrentHealth (- (Variables|Default|GetEnemyCurrentHealth) _returnvalue_3)))
  (if (<= (Variables|Default|GetEnemyCurrentHealth) 0.0)
    (Pawn|Components|CharacterMovement|DisableMovement (Variables|Character|GetCharacterMovement))
    (Collision|SetCollisionEnabled (Variables|Default|GetDragonCollision) "NoCollision")
    (Collision|SetCollisionEnabled (Variables|Character|GetMesh) "NoCollision")
    (Collision|SetCollisionEnabled (Variables|Collision|GetCapsuleComponent) "NoCollision")
    (Collision|SetCollisionEnabled (Variables|Default|GetMesh_ForestMonster) "NoCollision")
    (Rendering|SetVisibility (Variables|Default|GetWidget) false false)
    (switch Utilities|FlowControl|Switch|SwitchonE_ForestMonsterType (Variables|Default|GetForestMonsterType)
      (:NewEnumerator0
        (Utilities|FlowControl|DoOnce false
          (:Completed
            (Game|SpawnActorfromClass "/Game/Blueprints/Pickups/BP_Coin.BP_Coin_C" _returnvalue_2 "Undefined" 0 0))))
      (:NewEnumerator1
        (Utilities|FlowControl|DoOnce false
          (:Completed
            (Game|SpawnActorfromClass "/Game/Blueprints/Pickups/BP_apple.BP_apple_C" _returnvalue_2 "Undefined" 0 0 :!label _label))))
      (:NewEnumerator2
        (Utilities|FlowControl|DoOnce false
          (:Completed
            (Game|SpawnActorfromClass "/Game/Blueprints/Pickups/BP_Donut.BP_Donut_C" _returnvalue_2 "Undefined" 0 0))))
      (:NewEnumerator3
        (Utilities|FlowControl|DoOnce false
          (:Completed
            (goto _label)))))
    (Animation|Montage|PlayMontage (Variables|Character|GetMesh) "/Game/Convert/Enemy/Dragon03/Dragon_Death.Dragon_Death"
      (:then
        (Utilities|FlowControl|Delay 3.0)
        (Actor|DestroyActor)
        (bind _asbp_player_character (Utilities|Casting|CastToBP_PlayerCharacter (Game|GetPlayerCharacter 0)))
        (bind _aswbp_player (Utilities|Casting|CastToWBP_Player (Variables|/Script/TopdownShootingGame.PlayerCharacter|GetPlayerWidget _asbp_player_character)))
        (Default|IncreaseKillCount _aswbp_player)))
    (else
      (Default|UpdateEnemyHealthPercentage (Variables|Default|GetAs%20WBP%20Enemy%20Health) (/ _output_get (Variables|Default|GetEnemyMaxHealth)))
      (Audio|PlaySoundatLocation "/Engine/EditorSounds/GamePreview/EjectFromPlayer_Cue.EjectFromPlayer_Cue" (Transformation|GetActorLocation) "0, 0, 0" 1.0 1.0 0.0 0 0 0 0)
      (CallFunction|EnemyFlashingEffect)
      (Default|PlayDamageNumberAnimation (Variables|Default|GetAs%20WBP%20Enemy%20Health) _returnvalue_3))))

(fn ConstructionScript
  (bind _returnvalue (Rendering|Material|CreateDynamicMaterialInstance (Variables|Character|GetMesh) 0 "/Game/Blueprints/Enemies/M_ForestMonster.M_ForestMonster" "None" :!class /Script/Engine.PrimitiveComponent))
  (bind _output_get (Variables|Default|SetRef_Material _returnvalue))
  (Rendering|Material|SetMaterial (Variables|Default|GetMesh_ForestMonster) 0 _output_get))